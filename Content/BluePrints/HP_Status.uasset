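; HP_Status is a Blueprint that holds max and current hit point values and formats them for HUD display.
; SetHP writes both values directly, without clamping.
; GetStatsForHUD returns them as truncated whole-number text, plus current HP normalized against max HP for a progress bar.
; The event graph has no active logic, so values change only through calls from outside.
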(fn `GetStatsForHUD`
  (returns (`Max HP` :type Text) (`Current HP` :type Text) (`HP Progress Bar` :type "Float (double-precision)"))
  (bind _max_hp (`self.Max HP`))
  (bind _current_hp (`self.Current HP`))
  (return (`KismetTextLibrary.Conv_IntToText` (`KismetMathLibrary.FTrunc` _max_hp)) (`KismetTextLibrary.Conv_IntToText` (`KismetMathLibrary.FTrunc` _current_hp)) (`KismetMathLibrary.NormalizeToRange` _current_hp 0.0 _max_hp)))

(fn `Set HP`
  (params (`Set Max HP` :type "Float (double-precision)") (`Set Current HP` :type "Float (double-precision)"))
  (set `self.Max HP` `Set Max HP`)
  (set `self.Current HP` `Set Current HP`))