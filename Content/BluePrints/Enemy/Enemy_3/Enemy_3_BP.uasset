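; Enemy_3 character Blueprint for a melee enemy with health, headshot damage and ragdoll death.
; Attack events freeze movement and play a montage while both it and the player live, then restore speed.
; Toggled right-hand collision deals random damage once per swing.
; Incoming damage is multiplied on head hits; a looping timer polls health to trigger ragdoll and delayed destruction.
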(event `self.ReceiveBeginPlay`
  (`self.Set Health`)
  (set `self.Start Speed` (`CharacterMovementComponent.MaxWalkSpeed` (`self.CharacterMovement`))))

(event `/Game/BluePrints/Character/BPI_Take_Damage.TakingDamage`
  (params (Bone :type Name) (Damage :type "Float (single-precision)") (Instrigator :type "Actor Object Reference"))
  (`self.Calculate Damage` Bone Damage Instrigator))

(event `Event Destroy`
  (params (Delay :type "Float (double-precision)") (Target :type "Actor Object Reference"))
  (`self.Destroy Macros` Delay Target))

(event `Attacking Start`
  (`KismetSystemLibrary.PrintString` "Атака" true true (struct :`R` 1.0 :`B` 0.829394 :`A` 1.0) 5.0)
  (if (and (not (`/Game/BluePrints/Character/HP_Status.Is Dead` (`/Game/BluePrints/Character/PlayerCharacter_BP.HP_Status` (cast `/Game/BluePrints/Character/PlayerCharacter_BP` (`GameplayStatics.GetPlayerCharacter` 0) :!pure true)))) (not (`self.is Dead`)))
    (`/Engine/EditorBlueprintResources/StandardMacros.DoOnce` false :!label _label
      (:`Completed`
        (set `CharacterMovementComponent.MaxWalkSpeed` 0.0 (`self.CharacterMovement`))
        (`self.PlayAnimMontage` "/Game/Anim/Enemy/Enemy_3/Enemy_3_Attack_Montage.Enemy_3_Attack_Montage" 2.0)))))

(event `Attacking End`
  (set `CharacterMovementComponent.MaxWalkSpeed` (`self.Start Speed`) (`self.CharacterMovement`))
  (goto _label :!via `Reset`))

(event `EnableRightHandColision`
  (`PrimitiveComponent.SetCollisionEnabled` (`self.RightHend`) "QueryOnly"))

(event `DisableRightHandColision`
  (`PrimitiveComponent.SetCollisionEnabled` (`self.RightHend`) "NoCollision")
  (`self.RefreashRighttHendAttack`))

(event `self.RightHend.OnComponentBeginOverlap`
  (params (OverlappedComponent :type "PrimitiveComponent Object Reference") (OtherActor :type "Actor Object Reference") (OtherComp :type "PrimitiveComponent Object Reference") (OtherBodyIndex :type Integer) (bFromSweep :type Boolean) (SweepResult :type "HitResult Structure (by ref)"))
  (if (!= OtherActor self)
    (`/Engine/EditorBlueprintResources/StandardMacros.DoOnce` false :!label _label_2
      (:`Completed`
        (`GameplayStatics.ApplyDamage` OtherActor (`KismetMathLibrary.RandomFloatInRange` 50.0 100.0))))))

(event `RefreashRighttHendAttack`
  (goto _label_2 :!via `Reset`))

(fn `Calculate Damage`
  (params (Bone :type Name) (Damage :type "Float (double-precision)") (Instigator :type "Actor Object Reference"))
  (locals (DamageLocal :type "Float (double-precision)"))
  (set `local.DamageLocal` Damage)
  (if (== Bone "head")
    (set `self.Current Health` (- (`self.Current Health`) (* (`local.DamageLocal`) 10.0)))
    (else
      (set `self.Current Health` (- (`self.Current Health`) (`local.DamageLocal`))))))

(fn `Death`
  (locals (`Time Delay` :type "Float (double-precision)" :default 3.0))
  (bind _mesh (`self.Mesh`))
  (if (< (`self.Current Health`) 0.0)
    (set `self.is Dead` true)
    (`SkeletalMeshComponent.SetAllBodiesSimulatePhysics` _mesh true)
    (`PrimitiveComponent.SetCollisionProfileName` _mesh "Ragdoll" true)
    (`PrimitiveComponent.SetCollisionEnabled` (`self.CapsuleComponent`) "NoCollision")
    (`KismetSystemLibrary.K2_PauseTimerHandle` (`self.Timer`))
    (`self.Event Destroy` (`local.Time Delay`) self)))

(fn `Set Health`
  (set `self.Current Health` (`self.Max Health`))
  (bind _returnvalue (`KismetSystemLibrary.K2_SetTimer` null "Death" 0.1 true))
  (set `self.Timer` _returnvalue))

(fn `UserConstructionScript`)