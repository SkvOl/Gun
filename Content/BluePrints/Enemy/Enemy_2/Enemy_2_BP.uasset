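; Enemy_2 mutant character with randomized left/right melee montages, health regeneration and ragdoll death.
; Attack events stop movement and toggle hand overlap collision for random damage, with DoOnce gates whose resets are crossed between hands.
; Incoming damage is multiplied for headshots, while a looping timer polls health to trigger ragdoll and delayed destruction.
; Delayed Tick logic regenerates and prints health, updating IsHide against a one-third health threshold.
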(event `self.ReceiveBeginPlay`
  (`self.Set Health`)
  (set `self.Start Speed` (`CharacterMovementComponent.MaxWalkSpeed` (`self.CharacterMovement`))))

(event `/Game/BluePrints/Character/BPI_Take_Damage.TakingDamage`
  (params (Bone :type Name) (Damage :type "Float (single-precision)") (Instrigator :type "Actor Object Reference"))
  (`self.Calculate Damage` Bone Damage Instrigator))

(event `Event Destroy`
  (params (Delay :type "Float (double-precision)") (Target :type "Actor Object Reference"))
  (`self.Destroy Macros` Delay Target))

(event `Attacking Start`
  (if (and (not (`/Game/BluePrints/Character/HP_Status.Is Dead` (`/Game/BluePrints/Character/PlayerCharacter_BP.HP_Status` (cast `/Game/BluePrints/Character/PlayerCharacter_BP` (`GameplayStatics.GetPlayerCharacter` 0) :!pure true)))) (not (`self.is Dead`)))
    (`/Engine/EditorBlueprintResources/StandardMacros.DoOnce` false :!label _label
      (:`Completed`
        (set `CharacterMovementComponent.MaxWalkSpeed` 0.0 (`self.CharacterMovement`))
        (if (`KismetMathLibrary.RandomBoolWithWeight` 0.5)
          (`self.PlayAnimMontage` "/Game/Anim/Enemy/Enemy_2/Mutant_Attack_left_Montage.Mutant_Attack_left_Montage")
          (else
            (`self.PlayAnimMontage` "/Game/Anim/Enemy/Enemy_2/Mutant_Attack_Right_Montage.Mutant_Attack_Right_Montage")))))))

(event `Attacking End`
  (set `CharacterMovementComponent.MaxWalkSpeed` (`self.Start Speed`) (`self.CharacterMovement`))
  (goto _label :!via `Reset`))

(event `EnableRightHandColision`
  (`PrimitiveComponent.SetCollisionEnabled` (`self.RightHend`) "QueryOnly"))

(event `DisableRightHandColision`
  (`PrimitiveComponent.SetCollisionEnabled` (`self.RightHend`) "NoCollision")
  (`self.RefreashRightHendAttack`))

(event `EnableLeftHandColision`
  (`PrimitiveComponent.SetCollisionEnabled` (`self.LeftHend`) "QueryOnly"))

(event `DisableLeftHandColision`
  (`PrimitiveComponent.SetCollisionEnabled` (`self.LeftHend`) "NoCollision")
  (`self.RefreashLeftHendAttack`))

(event `self.RightHend.OnComponentBeginOverlap`
  (params (OverlappedComponent :type "PrimitiveComponent Object Reference") (OtherActor :type "Actor Object Reference") (OtherComp :type "PrimitiveComponent Object Reference") (OtherBodyIndex :type Integer) (bFromSweep :type Boolean) (SweepResult :type "HitResult Structure (by ref)"))
  (if (!= OtherActor self)
    (`/Engine/EditorBlueprintResources/StandardMacros.DoOnce` false :!label _label_2
      (:`Completed`
        (`GameplayStatics.ApplyDamage` OtherActor (`KismetMathLibrary.RandomFloatInRange` 50.0 100.0))))))

(event `RefreashLeftHendAttack`
  (goto _label_2 :!via `Reset`))

(event `self.LeftHend.OnComponentBeginOverlap`
  (params (OverlappedComponent :type "PrimitiveComponent Object Reference") (OtherActor :type "Actor Object Reference") (OtherComp :type "PrimitiveComponent Object Reference") (OtherBodyIndex :type Integer) (bFromSweep :type Boolean) (SweepResult :type "HitResult Structure (by ref)"))
  (if (!= OtherActor self)
    (`/Engine/EditorBlueprintResources/StandardMacros.DoOnce` false :!label _label_3
      (:`Completed`
        (`GameplayStatics.ApplyDamage` OtherActor (`KismetMathLibrary.RandomFloatInRange` 50.0 100.0))))))

(event `RefreashRightHendAttack`
  (goto _label_3 :!via `Reset`))

(event `self.ReceiveTick`
  (params (DeltaSeconds :type "Float (single-precision)"))
  ;[1 1 1] Регенерация
  (`KismetSystemLibrary.PrintString` (`KismetStringLibrary.Conv_DoubleToString` (`self.Current Health`)))
  (`KismetSystemLibrary.Delay` 0.2)
  (if (< (`self.Current Health`) (`self.Max Health`))
    (set `self.Current Health` (+ (`self.Current Health`) 1.0))
    (if (<= (`self.Current Health`) (/ (`self.Max Health`) 3.0))
      (set `self.Is Hide` true)
      (else
        (set `self.Is Hide` false)))))

(fn `Calculate Damage`
  (params (Bone :type Name) (Damage :type "Float (double-precision)") (Instigator :type "Actor Object Reference"))
  (locals (DamageLocal :type "Float (double-precision)"))
  (set `local.DamageLocal` Damage)
  (if (== Bone "head")
    (set `self.Current Health` (- (`self.Current Health`) (* (`local.DamageLocal`) 10.0)))
    (else
      (set `self.Current Health` (- (`self.Current Health`) (`local.DamageLocal`))))))

(fn `Death`
  (locals (`Time Delay` :type "Float (double-precision)" :default 3.0))
  (bind _mesh (`self.Mesh`))
  (if (< (`self.Current Health`) 0.0)
    (set `self.is Dead` true)
    (`SkeletalMeshComponent.SetAllBodiesSimulatePhysics` _mesh true)
    (`PrimitiveComponent.SetCollisionProfileName` _mesh "Ragdoll" true)
    (`PrimitiveComponent.SetCollisionEnabled` (`self.CapsuleComponent`) "NoCollision")
    (`KismetSystemLibrary.K2_PauseTimerHandle` (`self.Timer`))
    (`self.Event Destroy` (`local.Time Delay`) self)))

(fn `Set Health`
  (set `self.Current Health` (`self.Max Health`))
  (bind _returnvalue (`KismetSystemLibrary.K2_SetTimer` null "Death" 0.1 true))
  (set `self.Timer` _returnvalue))

(fn `UserConstructionScript`)