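; Base weapon Blueprint that loads its stats from DT_Weapon by row name and handles firing, ammo and reloading.
; FirePress runs single, burst or auto fire, gated by firing, fire-delay and reload flags.
; Each shot traces from the aiming or character camera, spawns a randomly angled Bullet_BP from the muzzle, plays montages and applies recoil.
; An empty clip triggers reload montages and delay, while a separate ReloadWeapon event transfers reserve ammo.
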(event `FirePress`
  (params (TrigerBullet :type Boolean))
  (set `self.firing` TrigerBullet)
  (switch `/Game/BluePrints/Weapon/EnumFireMode` (`self.Fire Mode`)
    (:`NewEnumerator0`
      (if (`self.Can Shoot`)
        (set `self.FireRateDelay` true)
        (`self.SpawnProjectle`)
        (`KismetSystemLibrary.RetriggerableDelay` (`self.Fire Delay`))
        (set `self.FireRateDelay` false)
        (set `self.firing` false)))
    (:`NewEnumerator1`
      (if (`self.Can Shoot`)
        (if (> (`.BulletsBirst_38_36422A614B91B9A574343189F2BE6AB1` (break `/Game/BluePrints/Weapon/StructWeaponData` (`self.WeaponData`))) (`self.Current Buiiets Wirst`)) :!label _label
          (set `self.FireRateDelay` true)
          (`/Engine/EditorBlueprintResources/StandardMacros.IncrementInt` (`self.Current Buiiets Wirst`)
            (:`  `
              (`self.SpawnProjectle`)
              (`KismetSystemLibrary.RetriggerableDelay` (`self.Fire Delay`))
              (set `self.FireRateDelay` false)
              (goto _label)))
          (else
            (set `self.Current Buiiets Wirst` 0)
            (set `self.firing` false)))))
    (:`NewEnumerator2`
      (if (`self.Can Shoot`) :!label _label_2
        (set `self.FireRateDelay` true)
        (`self.SpawnProjectle`)
        (`KismetSystemLibrary.RetriggerableDelay` (`self.Fire Delay`))
        (set `self.FireRateDelay` false)
        (goto _label_2)))))

(event `AutoReload`
  (bind ((`AmmoMax_16_B0C6717C45456B126EDE7AA096FC9619` _ammomax) (`CurrentAmmo_20_50B9549845FAC27363F98CAE4057A077` _currentammo)) (break `/Game/BluePrints/Weapon/StructWeaponData` (`self.WeaponData`)))
  (if (== _currentammo 0)
    (if (not (== _ammomax 0))
      (set `self.IsReloading` true)
      (`self.Reloading`)
      (`KismetSystemLibrary.Delay` (`.ReloadDellay_7_D1EE58EF4F56B61D204126B7664481C7` (break `/Game/BluePrints/Weapon/StructWeaponData` (`self.WeaponData`))))
      (set `self.IsReloading` false))))

(event `Reloading`
  (bind ((`AmmoMax_16_B0C6717C45456B126EDE7AA096FC9619` _ammomax) (`AmmoinClip_18_2C591B314B7D27F8E020B1BF08927AA7` _ammoinclip) (`CurrentAmmo_20_50B9549845FAC27363F98CAE4057A077` _currentammo)) (break `/Game/BluePrints/Weapon/StructWeaponData` (`self.WeaponData`)))
  (if (== _ammomax 0)
    _
    (elif (not (== _ammoinclip _currentammo))
      (bind _output_get (set `self.IsReloading` true))
      (if _output_get
        (`self.PlayMontage` (`.ReloadMontage_26_ECFE6A4F42D51212D9B15DA15EFB8E5E` (break `/Game/BluePrints/Weapon/StructWeaponData` (`self.WeaponData`))) "/Game/Anim/AnimStarterPack/Montage/Reload_Rifle_Hip_Montage.Reload_Rifle_Hip_Montage")
        (`KismetSystemLibrary.Delay` (`.ReloadDellay_7_D1EE58EF4F56B61D204126B7664481C7` (break `/Game/BluePrints/Weapon/StructWeaponData` (`self.WeaponData`))))
        (set `self.IsReloading` false)))))

(event `ReloadWeapon`
  (bind ((`AmmoMax_16_B0C6717C45456B126EDE7AA096FC9619` _ammomax) (`AmmoinClip_18_2C591B314B7D27F8E020B1BF08927AA7` _ammoinclip) (`CurrentAmmo_20_50B9549845FAC27363F98CAE4057A077` _currentammo)) (break `/Game/BluePrints/Weapon/StructWeaponData` (`self.WeaponData`)))
  (bind (_firemode _muzzlename _firerate _reloaddellay _weapolspaite _mindamage _maxdamage _ammomax_2 _ammoinclip_2 _currentammo_2 _firingmotage _reloadmontage _weapon_recoel _bulletsbirst _birsttype _bulletsinshoot _canscop) (break `/Game/BluePrints/Weapon/StructWeaponData` (`self.WeaponData`)))
  (if (> _ammomax 0)
    (set `self.NeedArmmor` (- _ammoinclip _currentammo))
    (if (<= (`.AmmoMax_16_B0C6717C45456B126EDE7AA096FC9619` (break `/Game/BluePrints/Weapon/StructWeaponData` (`self.WeaponData`))) (`self.NeedArmmor`))
      (set `self.WeaponData` (make `/Game/BluePrints/Weapon/StructWeaponData` _firemode _muzzlename _firerate _reloaddellay _weapolspaite _mindamage _maxdamage 0 _ammoinclip_2 (+ _currentammo_2 _ammomax_2)))
      (else
        (set `self.WeaponData` (make `/Game/BluePrints/Weapon/StructWeaponData` _firemode _muzzlename _firerate _reloaddellay _weapolspaite _mindamage _maxdamage (- _ammomax_2 (`self.NeedArmmor`)) _ammoinclip_2 _ammoinclip_2 _firingmotage _reloadmontage _weapon_recoel _bulletsbirst _birsttype _bulletsinshoot _canscop))))))

(fn `Calculate Direction`
  (returns (Location :type "Vector Structure") (Rotation :type "Rotator Structure"))
  (bind _returnvalue (`self.MuzzlePosition`))
  (bind _charref (`self.CharRef`))
  (bind (_returnvalue_location _returnvalue_rotation) (`KismetMathLibrary.BreakTransform` (`SceneComponent.K2_GetComponentToWorld` (select `bool` (`/Game/BluePrints/Character/PlayerCharacter_BP.Aiming` _charref) :`false` (`/Game/BluePrints/Character/PlayerCharacter_BP.1` _charref) :`true` (`self.Weapon_Camera`)))))
  (bind _returnvalue_2 (+ _returnvalue_location (* (`KismetMathLibrary.GetForwardVector` _returnvalue_rotation) 100000.0)))
  (bind (_outhit _returnvalue_3) (`KismetSystemLibrary.LineTraceSingleForObjects` (+ _returnvalue_location (* (`KismetMathLibrary.GetForwardVector` _returnvalue_rotation) (`KismetMathLibrary.VSize` (- _returnvalue_location (`self.MuzzlePosition`))))) _returnvalue_2 (`|MakeArray` "ObjectTypeQuery1" :!type "EObjectTypeQuery Enum")))
  (return _returnvalue (`KismetMathLibrary.FindLookAtRotation` _returnvalue (`KismetMathLibrary.SelectVector` (`.ImpactPoint` (`GameplayStatics.BreakHitResult` _outhit)) _returnvalue_2 _returnvalue_3))))

(fn `CalculateFinaleDirection`
  (params (Location :type "Vector Structure") (Rotation :type "Rotator Structure"))
  (returns (Transform :type "Transform Structure"))
  (bind _returnvalue (* (`self.Weapol Spaite`) -1.0))
  (return (`KismetMathLibrary.MakeTransform` Location (`KismetMathLibrary.ComposeRotators` Rotation (`KismetMathLibrary.MakeRotator` (`KismetMathLibrary.RandomFloatInRange` _returnvalue) (`KismetMathLibrary.RandomFloatInRange` _returnvalue) (`KismetMathLibrary.RandomFloatInRange` _returnvalue))))))

(fn `Can Shoot`
  (returns (Retern :type Boolean))
  (return (and (`self.firing`) (not (`self.FireRateDelay`)) (not (`self.IsReloading`)))))

(fn `Hes Ammo`
  (returns (Teark :type Boolean))
  (return (> (`.CurrentAmmo_20_50B9549845FAC27363F98CAE4057A077` (break `/Game/BluePrints/Weapon/StructWeaponData` (`self.WeaponData`))) 0)))

(fn `PlayMontage`
  (params (WeaponAnimy :type "AnimMontage Object Reference") (CharacterAnim :type "AnimMontage Object Reference"))
  (`AnimInstance.Montage_Play` (`SkeletalMeshComponent.GetAnimInstance` (`self.WeaponMesh`)) WeaponAnimy 1.0 "MontageLength" 0.0 true)
  (`AnimInstance.Montage_Play` (`SkeletalMeshComponent.GetAnimInstance` (`Character.Mesh` (`self.CharRef`))) CharacterAnim 1.0 "MontageLength" 0.0 true))

(fn `SpawnProjectle`
  (bind ((`MinDamage_11_5C26D20749606B8AF5695C8900A259BF` _mindamage) (`MaxDamage_13_288C34464762309E88159E9CF3E5300F` _maxdamage)) (break `/Game/BluePrints/Weapon/StructWeaponData` (`self.WeaponData`)))
  (bind (_firemode _muzzlename _firerate _reloaddellay _weapolspaite _mindamage_2 _maxdamage_2 _ammomax _ammoinclip _currentammo _firingmotage _reloadmontage _weapon_recoel _bulletsbirst _birsttype _bulletsinshoot _canscop) (break `/Game/BluePrints/Weapon/StructWeaponData` (`self.WeaponData`)))
  (if (`self.Hes Ammo`)
    (`self.PlayMontage` (`.firingMotage_25_E9EFC8344916BAADFD67C59C8EFB2417` (break `/Game/BluePrints/Weapon/StructWeaponData` (`self.WeaponData`))) (select `bool` (`/Game/BluePrints/Character/PlayerCharacter_BP.Aiming` (`self.CharRef`)) :`false` "/Game/Anim/AnimStarterPack/Montage/Fire_Rifle_Hip_Montage.Fire_Rifle_Hip_Montage" :`true` "/Game/Anim/AnimStarterPack/Montage/Fire_Rifle_Ironsights_Montage.Fire_Rifle_Ironsights_Montage" :!type "AnimMontage Object Reference"))
    (bind (_location _rotation) (`self.Calculate Direction`))
    (bind _transform (`self.CalculateFinaleDirection` _location _rotation))
    (`|SpawnActorFromClass` "/Game/BluePrints/Weapon/Bullet_BP.Bullet_BP_C" _transform "Undefined" "OverrideRootScale" null (`KismetMathLibrary.RandomFloatInRange` _mindamage _maxdamage) null)
    (`/Game/BluePrints/Character/PlayerCharacter_BP.Weapon ReCoel` (`self.CharRef`) (`.Weapon_Recoel_37_4B48537D492432D0B6C59B97B07FEBFE` (break `/Game/BluePrints/Weapon/StructWeaponData` (`self.WeaponData`))))
    (set `self.WeaponData` (make `/Game/BluePrints/Weapon/StructWeaponData` _firemode _muzzlename _firerate _reloaddellay _weapolspaite _mindamage_2 _maxdamage_2 _ammomax _ammoinclip (- _currentammo 1) _firingmotage _reloadmontage _weapon_recoel _bulletsbirst _birsttype 0 _canscop))
    (else
      (`self.AutoReload`))))

(fn `UserConstructionScript`
  (locals (NewLocalVar_0 :type "Float (double-precision)") (FireMode :type "/Game/BluePrints/Weapon/EnumFireMode Enum") (MuzzleName :type Name) (FireRate :type "Float (double-precision)") (ReloadDellay :type "Float (double-precision)") (WeaponSpraite :type "Float (double-precision)"))
  (bind _returnvalue (`|GetDataTableRow` "/Game/BluePrints/Weapon/DT_Weapon.DT_Weapon" (`self.WeaponRowName`))
    (:`then`
      (bind _output_get (set `self.WeaponData` _returnvalue))
      (bind (_firemode _muzzlename _firerate _reloaddellay _weapolspaite _mindamage _maxdamage _ammomax _ammoinclip _currentammo _firingmotage _reloadmontage _weapon_recoel _bulletsbirst _birsttype) (break `/Game/BluePrints/Weapon/StructWeaponData` _output_get))
      (set `local.FireMode` _firemode)
      (set `local.MuzzleName` _muzzlename)
      (set `local.FireRate` _firerate)
      (set `local.ReloadDellay` _reloaddellay)
      (set `local.WeaponSpraite` _weapolspaite)
      (set `self.Bullets Birst` _bulletsbirst)
      (set `self.Birst Type` _birsttype)
      (set `self.Weapon Recoel` _weapon_recoel))))